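; BP_Enemy is a short-lived enemy actor that damages the player on contact and awards score when shot, expiring on its own after a fixed lifespan.
; Overlapping BP_Player subtracts health, prints it, updates the health bar, destroys the enemy, and at zero health flags the player dead and shows restart.
; A component overlap with BP_projectile adds score to that projectile's player, refreshes the score widget and destroys the enemy.
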(event OnComponentBeginOverlap(BP_Enemy)
  (params (OverlappedComponent :type Primitive%20Component%20Object%20Reference) (OtherActor :type Actor%20Object%20Reference) (OtherComp :type Primitive%20Component%20Object%20Reference) (OtherBodyIndex :type Integer) (bFromSweep :type Boolean) (SweepResult :type Hit%20Result%20Structure%20%28by%20ref%29))
  (bind _asbp_projectile (Utilities|Casting|CastToBP_projectile OtherActor))
  (Variables|/Game/InfiniteMatrix/Blueprints/BP_Player.BP_Player_C|SetScore (Variables|/Game/InfiniteMatrix/Blueprints/BP_projectile.BP_projectile_C|GetNewPlayer _asbp_projectile) (+ (Variables|/Game/InfiniteMatrix/Blueprints/BP_Player.BP_Player_C|GetScore (Variables|/Game/InfiniteMatrix/Blueprints/BP_projectile.BP_projectile_C|GetNewPlayer _asbp_projectile)) 2e+01))
  (Default|UpdateScore (Variables|/Game/InfiniteMatrix/Blueprints/BP_Player.BP_Player_C|GetWB_HealthBar (Variables|/Game/InfiniteMatrix/Blueprints/BP_projectile.BP_projectile_C|GetNewPlayer _asbp_projectile)))
  (Actor|DestroyActor))

(event EventBeginPlay
  (Actor|SetLifeSpan 1e+01))

(event Collision|EventActorBeginOverlap
  (params (OtherActor :type Actor%20Object%20Reference))
  (bind _asbp_player (Utilities|Casting|CastToBP_Player OtherActor))
  (bind _output_get (Variables|/Game/InfiniteMatrix/Blueprints/BP_Player.BP_Player_C|SetHealth _asbp_player (- (Variables|/Game/InfiniteMatrix/Blueprints/BP_Player.BP_Player_C|GetHealth _asbp_player) 2e+01)))
  (Development|PrintString (Utilities|String|ToString(Float) _output_get))
  (Default|UpdateHealthBar (Variables|/Game/InfiniteMatrix/Blueprints/BP_Player.BP_Player_C|GetWB_HealthBar _asbp_player) _output_get)
  (Actor|DestroyActor)
  (if (<= _output_get 0.0)
    (Variables|/Game/InfiniteMatrix/Blueprints/BP_Player.BP_Player_C|SetisDead _asbp_player true)
    (Default|DisplayRestart _asbp_player)))

(event EventTick
  (params (DeltaSeconds :type Float%20%28single-precision%29)))

(fn ConstructionScript)